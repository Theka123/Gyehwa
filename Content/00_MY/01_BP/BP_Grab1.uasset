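; BP_Grab1 is an actor whose static mesh changes color based on the component that overlaps it.
; On the mesh's begin overlap, a chain of tag checks on the other component picks the pink, blue, yellow or green material.
; The pink and blue branches also replace the mesh's component tags with the matching tag variable, while yellow and green change only the material.
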(event OnComponentBeginOverlap(StaticMesh)
  (params (OverlappedComponent :type Primitive%20Component%20Object%20Reference) (OtherActor :type Actor%20Object%20Reference) (OtherComp :type Primitive%20Component%20Object%20Reference) (OtherBodyIndex :type Integer) (bFromSweep :type Boolean) (SweepResult :type Hit%20Result%20Structure%20%28by%20ref%29))
  (if (Components|ComponentHasTag OtherComp "Pink")
    (Rendering|Material|SetMaterial (Variables|Default|GetStaticMesh) 0 "/Game/00_MY/03_Materials/M_Pink.M_Pink")
    (Variables|/Script/Engine.ActorComponent|SetComponentTags (Variables|Default|GetStaticMesh) (Variables|Default|GetTag_Pink))
    (elif (Components|ComponentHasTag OtherComp "Blue")
      (Rendering|Material|SetMaterial (Variables|Default|GetStaticMesh) 0 "/Game/00_MY/03_Materials/M_Blue.M_Blue")
      (Variables|/Script/Engine.ActorComponent|SetComponentTags (Variables|Default|GetStaticMesh) (Variables|Default|GetTag_Blue))
      (elif (Components|ComponentHasTag OtherComp "Yellow")
        (Rendering|Material|SetMaterial (Variables|Default|GetStaticMesh) 0 "/Game/00_MY/03_Materials/M_Yellow.M_Yellow")
        (elif (Components|ComponentHasTag OtherComp "Green")
          (Rendering|Material|SetMaterial (Variables|Default|GetStaticMesh) 0 "/Game/00_MY/03_Materials/M_Green.M_Green"))))))

(event EventBeginPlay)

(event Collision|EventActorBeginOverlap
  (params (OtherActor :type Actor%20Object%20Reference)))

(fn ConstructionScript)