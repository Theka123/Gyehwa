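; BP_testblock is a test Blueprint of four cubes that get painted when a brush touches them.
; Each cube is paired with a box component whose begin-overlap event checks the other component for the "brush" tag.
; On a match, the paired cube's first material slot switches to its own fixed color material, with nothing in the graph to revert it.
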(event OnComponentBeginOverlap(Box1)
  (params (OverlappedComponent :type Primitive%20Component%20Object%20Reference) (OtherActor :type Actor%20Object%20Reference) (OtherComp :type Primitive%20Component%20Object%20Reference) (OtherBodyIndex :type Integer) (bFromSweep :type Boolean) (SweepResult :type Hit%20Result%20Structure%20%28by%20ref%29))
  (if (Components|ComponentHasTag OtherComp "brush")
    (Rendering|Material|SetMaterial (Variables|Default|GetCube1) 0 "/Game/00_MY/03_Materials/M_Pink.M_Pink")))

(event OnComponentBeginOverlap(Box)
  (params (OverlappedComponent :type Primitive%20Component%20Object%20Reference) (OtherActor :type Actor%20Object%20Reference) (OtherComp :type Primitive%20Component%20Object%20Reference) (OtherBodyIndex :type Integer) (bFromSweep :type Boolean) (SweepResult :type Hit%20Result%20Structure%20%28by%20ref%29))
  (if (Components|ComponentHasTag OtherComp "brush")
    (Rendering|Material|SetMaterial (Variables|Default|GetCube) 0 "/Game/00_MY/03_Materials/M_Blue.M_Blue")))

(event OnComponentBeginOverlap(Box2)
  (params (OverlappedComponent :type Primitive%20Component%20Object%20Reference) (OtherActor :type Actor%20Object%20Reference) (OtherComp :type Primitive%20Component%20Object%20Reference) (OtherBodyIndex :type Integer) (bFromSweep :type Boolean) (SweepResult :type Hit%20Result%20Structure%20%28by%20ref%29))
  (if (Components|ComponentHasTag OtherComp "brush")
    (Rendering|Material|SetMaterial (Variables|Default|GetCube2) 0 "/Game/00_MY/03_Materials/M_Yellow.M_Yellow")))

(event OnComponentBeginOverlap(Box3)
  (params (OverlappedComponent :type Primitive%20Component%20Object%20Reference) (OtherActor :type Actor%20Object%20Reference) (OtherComp :type Primitive%20Component%20Object%20Reference) (OtherBodyIndex :type Integer) (bFromSweep :type Boolean) (SweepResult :type Hit%20Result%20Structure%20%28by%20ref%29))
  (if (Components|ComponentHasTag OtherComp "brush")
    (Rendering|Material|SetMaterial (Variables|Default|GetCube3) 0 "/Game/00_MY/03_Materials/M_Green.M_Green")))

(fn ConstructionScript)